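; BP_SurgicalLight is a hanging surgical lamp that sways and flickers.
; The construction script snaps the lamp head to the cable's end, and a looping delay applies random horizontal forces to the cable.
; A second loop rolls a random number against FlickerFrequency to toggle the spotlight and swap the bulb material between glass and emissive.
; A gate makes the noise play only when the light comes back on.
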(event EventBeginPlay
  (bind _spotlight (Variables|Default|GetSpotLight))
  (bind _lamp_head (Variables|Default|GetLamp%20Head))
  (Utilities|FlowControl|Sequence
    (:then_0
      ;[1 1 1] Nudging
      (Utilities|FlowControl|Delay 0.2 :!label _label)
      (Variables|/Script/CableComponent.CableComponent|SetCableForce (Variables|Default|GetCable) (Math|Vector|MakeVector (Math|Random|RandomFloatinRange -5e+01 5e+01) (Math|Random|RandomFloatinRange -5e+01 5e+01) 0.0))
      (goto _label))
    (:then_1
      ;[1 1 1] Flickering Light
      (Math|Integer|CompareInt (Math|Random|RandomInteger 200) (Variables|Default|GetFlicker%20Frequency) :!label _label_2
        (:>
          (Rendering|SetVisibility _spotlight false false :!label _label_3)
          (Rendering|Material|SetMaterial _lamp_head 1 "/Game/Custom_Materials/M_Glass.M_Glass")
          (Utilities|FlowControl|Sequence
            (:then_0
              (goto _label_4 Open))
            (:then_1
              _)))
        (:==
          (goto _label_3))
        (:<
          (Rendering|SetVisibility _spotlight true false)
          (Utilities|FlowControl|Sequence
            (:then_0
              (Rendering|Material|SetMaterial _lamp_head 1 "/Game/Custom_Materials/EM_Fluorescent.EM_Fluorescent"))
            (:then_1
              (Utilities|FlowControl|Gate false :!label _label_4
                (:Exit
                  (Audio|Components|Audio|Play (Variables|Default|GetNoise) 0.0)
                  (goto _label_4 Close)))))))
      (Utilities|FlowControl|Delay 0.2)
      (goto _label_2))))

(fn ConstructionScript
  (Transformation|AttachComponentToComponent (Variables|Default|GetLamp%20Head) (Variables|Default|GetCable) "CableEnd" "SnapToTarget" "SnapToTarget" "KeepRelative" true))