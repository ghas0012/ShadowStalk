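; Fluorescent light Blueprint that flickers at random, with sound.
; From BeginPlay it loops every 0.2 seconds, comparing a random integer to FlickerFrequency to decide whether the light is on or off.
; Each state toggles the RectLight's visibility and swaps the mesh between emissive and glass materials.
; A gate reopens while lit and closes after playing FlickerNoise, so consecutive off ticks trigger the sound only once.
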(event EventBeginPlay
  (bind _rectlight (Variables|Default|GetRectLight))
  (Math|Integer|CompareInt (Math|Random|RandomInteger 200) (Variables|Default|GetFlicker%20Frequency) :!label _label
    (:>
      (Rendering|SetVisibility _rectlight true false :!label _label_2)
      (Rendering|Material|SetMaterial (Variables|Debug|GetStaticMeshComponent) 0 "/Game/Custom_Materials/EM_Fluorescent.EM_Fluorescent")
      (Utilities|FlowControl|Sequence
        (:then_0
          (goto _label_3 Open))
        (:then_1
          _)))
    (:==
      (goto _label_2))
    (:<
      (Rendering|SetVisibility _rectlight false false)
      (Utilities|FlowControl|Sequence
        (:then_0
          (Rendering|Material|SetMaterial (Variables|Debug|GetStaticMeshComponent) 0 "/Game/Custom_Materials/M_Glass.M_Glass"))
        (:then_1
          (Utilities|FlowControl|Gate false :!label _label_3
            (:Exit
              (Audio|Components|Audio|Play (Variables|Default|GetFlickerNoise) 0.0)
              (goto _label_3 Close)))))))
  (Utilities|FlowControl|Delay 0.2)
  (goto _label))

(fn ConstructionScript)